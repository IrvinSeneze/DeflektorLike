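; GM_Player manages the player's Energy and Overload values over time.
; On BeginPlay it starts two looping timers that call its update functions by name.
; The slower timer drains Energy steadily while it is above zero.
; The faster timer raises Overload toward OverloadMax while OverloadItemCount is positive, and otherwise lowers it toward zero, with no exact clamping at either limit.
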(event `self.ReceiveBeginPlay`
  (`KismetSystemLibrary.K2_SetTimer` null "gestionOverload" 0.1 true)
  (`KismetSystemLibrary.K2_SetTimer` null "gestionEnergy" 1.0 true))

(fn `gestionEnergy`
  (if (> (`self.Energy`) 0.0)
    (set `self.Energy` (- (`self.Energy`) 1.0))))

(fn `gestionOverload`
  (if (> (`self.OverloadItemCount`) 0)
    (if (< (`self.Overload`) (`self.OverloadMax`))
      (set `self.Overload` (+ (`self.Overload`) 6.0)))
    (elif (> (`self.Overload`) 0.0)
      (set `self.Overload` (- (`self.Overload`) 5.0)))))

(fn `UserConstructionScript`)