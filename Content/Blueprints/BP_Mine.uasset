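; BP_Mine is a laser-reactive object that counts toward the overload item total on the GM_Player game mode.
; Its LaserBounce function increments OverloadItemCount when the hit response is true and decrements it when false.
; An IsAdded flag guards both changes, so each mine is counted only once at a time.
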(fn `LaserBounce`
  (params (`P-LaserHit` :type "/Game/Blueprint/A_Laser Object Reference") (`P-HitResponse` :type Boolean) (`P-HitInformation` :type "HitResult Structure"))
  (returns (NewLaser :type "/Game/Blueprint/A_Laser Object Reference"))
  (bind _output_get (set `self.activate` `P-HitResponse`))
  (if _output_get
    (bind _asgm_player (cast `/Game/GM_Player` (`GameplayStatics.GetGameMode`)))
    (if (not (`self.isAdded`))
      (set `self.isAdded` true)
      (set `/Game/GM_Player.OverloadItemCount` (+ (`/Game/GM_Player.OverloadItemCount` _asgm_player) 1) _asgm_player))
    (return null)
    (else
      (bind _asgm_player_2 (cast `/Game/GM_Player` (`GameplayStatics.GetGameMode`)))
      (if (`self.isAdded`)
        (set `self.isAdded` false)
        (set `/Game/GM_Player.OverloadItemCount` (- (`/Game/GM_Player.OverloadItemCount` _asgm_player_2) 1) _asgm_player_2)
        (return null)))))

(fn `UserConstructionScript`)