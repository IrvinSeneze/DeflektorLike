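; Mirror actor for a laser mechanic that yaws automatically each tick or, with AutoRotation off, by left/right mouse clicks on its meshes.
; LaserBounce spawns an A_Laser at the impact point, oriented through CalculateRotation, inheriting color and source with an updated ID.
; It registers that laser with the mirror and source's child list.
; Without a hit response, it destroys attached lasers whose IDs contain the incoming ID.
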(event `self.ReceiveTick`
  (params (DeltaSeconds :type "Float (single-precision)"))
  (if (`self.Auto-Rotation`)
    (`SceneComponent.K2_AddWorldRotation` (`self.Miroir`) (`KismetMathLibrary.MakeRotator` 0.0 0.0 (`self.RotationValue`)) false false)))

(event `self.Miroir.OnClicked`
  (params (TouchedComponent :type "PrimitiveComponent Object Reference") (ButtonPressed :type "Key Structure"))
  (bind _rotationvalue (`self.RotationValue`))
  (bind _miroir (`self.Miroir`))
  (if (not (`self.Auto-Rotation`))
    (switch `string` (`KismetTextLibrary.Conv_TextToString` (`KismetInputLibrary.Key_GetDisplayName` ButtonPressed))
      (:`Left Mouse Button`
        (`SceneComponent.K2_AddWorldRotation` _miroir (`KismetMathLibrary.MakeRotator` 0.0 0.0 (* _rotationvalue -1.0)) false false :!label _label))
      (:`Right Mouse Button`
        (`SceneComponent.K2_AddWorldRotation` _miroir (`KismetMathLibrary.MakeRotator` 0.0 0.0 _rotationvalue) false false :!label _label_2)))))

(event `self.SM_Parent.OnClicked`
  (params (TouchedComponent :type "PrimitiveComponent Object Reference") (ButtonPressed :type "Key Structure"))
  (if (not (`self.Auto-Rotation`))
    (switch `string` (`KismetTextLibrary.Conv_TextToString` (`KismetInputLibrary.Key_GetDisplayName` ButtonPressed))
      (:`Left Mouse Button`
        (goto _label))
      (:`Right Mouse Button`
        (goto _label_2)))))

(fn `Clear Attached Lasers`
  (params (`P-IDClear` :type String))
  (bind (_arrayindex _arrayelement) (`/Engine/EditorBlueprintResources/StandardMacros.ReverseForEachLoop` (`self.LaserAttached`))
    (:`LoopBody`
      (`/Engine/EditorBlueprintResources/StandardMacros.IsValid` _arrayelement
        (:`Is Valid`
          (if (`KismetStringLibrary.Contains` (`/Game/Blueprint/A_Laser.Laser_ID` _arrayelement) (`local.P-IDClear`))
            (`self.K2_DestroyActor` _arrayelement)
            (`KismetArrayLibrary.Array_RemoveItem` (`self.LaserAttached`) _arrayelement)))))))

(fn `LaserBounce`
  (params (`P-LaserHit` :type "/Game/Blueprint/A_Laser Object Reference") (`P-HitResponse` :type Boolean) (`P-HitInformation` :type "HitResult Structure"))
  (returns (NewLaser :type "/Game/Blueprint/A_Laser Object Reference"))
  (bind _p_laserhit (`local.P-LaserHit`))
  (bind (_bblockinghit _binitialoverlap _time _distance _location _impactpoint _normal _impactnormal _physmat _hitactor _hitcomponent _hitbonename _bonename _hititem _elementindex _faceindex _tracestart) (`GameplayStatics.BreakHitResult` (`local.P-HitInformation`)))
  (if `P-HitResponse`
    (set `self.Active` true)
    (bind _returnvalue (`|SpawnActorFromClass` "/Game/Blueprint/A_Laser.A_Laser_C" (`KismetMathLibrary.MakeTransform` _impactpoint (`KismetMathLibrary.MakeRotFromZ` (`KismetMathLibrary.MirrorVectorByNormal` (- _impactpoint _tracestart) _impactnormal))) "Undefined" "MultiplyWithRoot" null (`/Game/Blueprint/A_Laser.Update ID` _p_laserhit "B") (`/Game/Blueprint/A_Lasers_Parents.LaserColor` _p_laserhit) (`/Game/Blueprint/A_Lasers_Parents.SpawnReference` _p_laserhit) null))
    (`KismetArrayLibrary.Array_Add` (`self.LaserAttached`) _returnvalue)
    (`KismetArrayLibrary.Array_Add` (`/Game/Blueprint/A_LaserSpawn.ChildLasers` (`/Game/Blueprint/A_Lasers_Parents.SpawnReference` (`local.P-LaserHit`))) _returnvalue)
    (return _returnvalue)
    (else
      (`self.Clear Attached Lasers` (`/Game/Blueprint/A_Laser.Laser_ID` (`local.P-LaserHit`)))
      (set `self.Active` false))))

(fn `UserConstructionScript`
  (`parent.UserConstructionScript`))