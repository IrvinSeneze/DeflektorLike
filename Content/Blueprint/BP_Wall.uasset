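; BP_Wall is a wall for a laser puzzle that changes color in response to laser hits.
; On BeginPlay it creates a dynamic material from Socle on SMParent and applies an initial color through PuzzleSolved.
; LaserBounce stores the hit response in Active and passes the laser's color to PuzzleSolved.
; PuzzleSolved sets the material's color parameter to the given color when Active, otherwise to a neutral grey.
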(event `self.ReceiveBeginPlay`
  (bind _returnvalue (`PrimitiveComponent.CreateDynamicMaterialInstance` (`self.SM_Parent`) 0 "/Game/Resources/socle.socle" "None"))
  (set `self.Material` _returnvalue)
  (`self.PuzzleSolved` (struct :`R` 0.31875 :`G` 0.29218 :`B` 0.255751 :`A` 1.0)))

(fn `LaserBounce`
  (params (`P-LaserHit` :type "/Game/Blueprint/A_Laser Object Reference") (`P-HitResponse` :type Boolean) (`P-HitInformation` :type "HitResult Structure"))
  (returns (NewLaser :type "/Game/Blueprint/A_Laser Object Reference"))
  (set `self.Active` `P-HitResponse`)
  (`self.PuzzleSolved` (`/Game/Blueprint/A_Lasers_Parents.LaserColor` `P-LaserHit`))
  (return null))

(fn `PuzzleSolved`
  (params (`Color Laser` :type "LinearColor Structure"))
  (`MaterialInstanceDynamic.SetVectorParameterValue` (`self.Material`) "param" (`KismetMathLibrary.SelectColor` `Color Laser` (struct :`R` 0.368627 :`G` 0.368627 :`B` 0.368627 :`A` 1.0) (`self.Active`))))

(fn `UserConstructionScript`)